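; Player pawn Blueprint, a task solution showing basic hand-built movement and jumping without CharacterMovementComponent.
; Tick calls Movement, which offsets the actor along world X and Y from forward/right input, scaled by speed and delta time.
; Jump applies a velocity-change impulse to the physics capsule while JumpCount is below MaxJumpCount, allowing multi-jumps.
; Capsule hits with an upward-facing normal reset JumpCount, serving as a simple landing check.
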(event `self.ReceiveTick`
  (params (DeltaSeconds :type "Float (single-precision)"))
  (`self.Movement`))

(event `InputAction|Jump`
  (params (Key :type "Key Structure"))
  (:`Pressed`
    ;[0 0 0] Check that we've not reached a max jump limit. This stops us being able to jump indefinitely and allows us to increase MaxJumpCount for features like double jump
    (if (< (`self.JumpCount`) (`self.MaxJumpCount`))
      ;[0 0 0] If we can jump, add impulse and increase the tracked JumpCount
      (`PrimitiveComponent.AddImpulse` (`self.Capsule`) (`KismetMathLibrary.MakeVector` 0.0 0.0 (`self.JumpForce`)) "None" true)
      (`/Engine/EditorBlueprintResources/StandardMacros.IncrementInt` (`self.JumpCount`)))))

(event `self.Capsule.OnComponentHit`
  (params (HitComponent :type "PrimitiveComponent Object Reference") (OtherActor :type "Actor Object Reference") (OtherComp :type "PrimitiveComponent Object Reference") (NormalImpulse :type "Vector Structure") (Hit :type "HitResult Structure (by ref)"))
  ;[0 0 0] If it's more than 0 then we've hit something below us. 1 is flat, anything between is a slope or at least hitting us from the side.
  ; Less than 0 to -1 means we're being hit from the side up to the top of the player "head".
  (if (> (.z (`.Normal` (`GameplayStatics.BreakHitResult` Hit))) 0.0)
    ;[0 0 0] If we've landed on a surface below us, reset jump count
    (set `self.JumpCount` 0)))

(fn `Movement`
  ;[0 0 0] A VERY simplified version of what's happening in the CharacterMovementComponent. Adding an offset to the current world location based on the inputs being pressed and the speeds being assigned. This is not using any of the ConsumeInput functionality so it's a basic form of the most manual way we can add movement to a default pawn
  (`self.K2_AddActorWorldOffset` (`KismetMathLibrary.MakeVector` (* (`self.GetInputAxisValue`) (* (`self.MoveSpeed`) (`GameplayStatics.GetWorldDeltaSeconds`))) (* (`self.GetInputAxisValue`) (* (`self.MoveSpeed`) (`GameplayStatics.GetWorldDeltaSeconds`))))))

(fn `UserConstructionScript`)