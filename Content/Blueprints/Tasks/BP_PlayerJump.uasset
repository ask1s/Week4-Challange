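; BP_PlayerJump is a player-controlled actor that moves along world X and Y and can perform a limited number of jumps.
; Tick offsets the actor by the forward and right input axes, scaled by move speed and delta time.
; Space applies a velocity-change impulse to the physics capsule while jumps remain and increments the count.
; Capsule hits with an upward-facing normal reset the jump count.
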(event `self.ReceiveTick`
  (params (DeltaSeconds :type "Float (single-precision)"))
  (`self.K2_AddActorWorldOffset` (`KismetMathLibrary.MakeVector` (* (`self.GetInputAxisValue`) (* (`self.MoveSpeed`) (`GameplayStatics.GetWorldDeltaSeconds`))) (* (`self.GetInputAxisValue`) (* (`self.MoveSpeed`) (`GameplayStatics.GetWorldDeltaSeconds`))))))

(event `Key|SpaceBar`
  (params (Key :type "Key Structure"))
  (:`Pressed`
    (if (< (`self.JumpCount`) (`self.MaxJumpsCount`))
      (`PrimitiveComponent.AddImpulse` (`self.Capsule`) (`KismetMathLibrary.MakeVector` 0.0 0.0 (`self.JumpForce`)) "None" true)
      (`/Engine/EditorBlueprintResources/StandardMacros.IncrementInt` (`KismetMathLibrary.Clamp` (`self.JumpCount`) 0 (`self.MaxJumpsCount`))))))

(event `self.Capsule.OnComponentHit`
  (params (HitComponent :type "PrimitiveComponent Object Reference") (OtherActor :type "Actor Object Reference") (OtherComp :type "PrimitiveComponent Object Reference") (NormalImpulse :type "Vector Structure") (Hit :type "HitResult Structure (by ref)"))
  (if (> (.z (`.Normal` (`GameplayStatics.BreakHitResult` Hit))) 0.0)
    (set `self.JumpCount` 0)))

(fn `UserConstructionScript`)